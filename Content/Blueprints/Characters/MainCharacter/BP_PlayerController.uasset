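; Player controller that sets up the local HUD and camera view when a match starts.
; OnStartMatch creates the WBP_PlayersLife widget from the passed player states, then after a short delay blends the view to the first BP_Camera found in the level.
; CastToPCs converts an array of controllers to BP_PlayerController references.
; The timer-based match-start polling is deprecated and disconnected.
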(event Custom|SetCameraPlayer
  (bind _outactors (Actor|GetAllActorsOfClass "/Game/Blueprints/Characters/MainCharacter/BP_Camera.BP_Camera_C"))
  (Game|Player|SetViewTargetwithBlend (Utilities|Array|Get(acopy) _outactors) 0.3 "VTBlend_Linear" 0.0 false))

(event Custom|CheckMatchStarted
  ;[1 1 1] deprecated
  (if (Class|GameModeBase|HasMatchStarted (Variables|Default|GetGame%20Mode))
    _))

(event EventBeginPlay)

(event EventOnStartMatch
  (params (PClocal :type S%20Player%20Controller%20Object%20Reference) (PlayerStates :type Array%20of%20S%20Player%20State%20Object%20References))
  (bind _returnvalue (UserInterface|CreateWidget "/Game/Blueprints/Widget/WBP_PlayersLife.WBP_PlayersLife_C" PClocal PlayerStates))
  (UserInterface|Viewport|AddtoViewport _returnvalue 0)
  (Utilities|FlowControl|Delay 1.0)
  (CallFunction|SetCameraPlayer))

(fn ConstructionScript)

(fn CasttoPCs
  (params (PcsIn :type Array%20of%20S%20Player%20Controller%20Object%20References))
  (for _array_element PcsIn
    (bind _asbp_player_controller (Utilities|Casting|CastToBP_PlayerController _array_element))
    (Utilities|Array|Add (LocalVariables|GetPcsOut) _asbp_player_controller))
  (return (LocalVariables|GetPcsOut)))
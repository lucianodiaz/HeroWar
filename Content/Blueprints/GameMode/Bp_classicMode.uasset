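; Classic-mode game mode that handles match start and respawns for multiplayer play.
; PostLogin collects player controllers and states, and ReadyToStartMatch reports true at two or more players.
; A looping timer calls StartMatch until the match has started, then multicasts the player states through SGameState.
; Killed actors are reused after a short delay: health is restored, then they move to a random PlayerStart and are unhidden.
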(event Custom|StartMatchHandler
  (if (Class|GameModeBase|HasMatchStarted)
    (Utilities|Time|ClearTimerbyFunctionName 0 "StartMatchHandler")
    (bind _assgame_state (Utilities|Casting|CastToSGameState (Game|GetGameState)))
    (Utilities|FlowControl|Delay 1.0)
    (Class|SGameState|MulticastonStartMatch _assgame_state (Variables|Default|GetPlayer%20States))
    (else
      (Class|GameMode|StartMatch))))

(event Custom|OnActorKilled_Event_0
  (params (VictimActor :type Actor%20Object%20Reference) (VictimController :type Controller%20Object%20Reference))
  (Utilities|IsValid VictimActor
    (:Is%20Valid
      (Utilities|FlowControl|Delay 2.0)
      (Class|SHealthComponent|Restore (Actor|GetComponentbyClass VictimActor "/Script/HeroWar.SHealthComponent"))
      (bind _outactors (Actor|GetAllActorsOfClass "/Script/Engine.PlayerStart"))
      (Transformation|SetActorLocation VictimActor (Transformation|GetActorLocation (Utilities|Array|Get(acopy) _outactors (Math|Random|RandomIntegerinRange 0 (- (Utilities|Array|Length _outactors) 1)))) false false)
      (Rendering|SetActorHiddenInGame VictimActor false))))

(event EventPostLogin
  (params (NewPlayer :type Player%20Controller%20Object%20Reference))
  (bind _asbp_player_controller (Utilities|Casting|CastToBP_PlayerController NewPlayer))
  (Utilities|Array|Add (Variables|Default|GetPlayerControllers) _asbp_player_controller)
  (bind _assplayer_state (Utilities|Casting|CastToSPlayerState (Variables|/Script/Engine.Controller|GetPlayerState _asbp_player_controller)))
  (Utilities|Array|Add (Variables|Default|GetPlayer%20States) _assplayer_state))

(event EventBeginPlay
  (EventDispatchers|AssignOnActorKilled (delegate Custom|OnActorKilled_Event_0))
  (Utilities|Time|SetTimerbyFunctionName 0 "StartMatchHandler" 1.0 true))

(fn ConstructionScript)

(fn ReadytoStartMatch
  (return (>= (Utilities|Array|Length (Variables|Default|GetPlayerControllers)) 2)))
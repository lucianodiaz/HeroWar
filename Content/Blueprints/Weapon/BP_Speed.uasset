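; BP_Speed is a timed speed power-up that makes the player's character move faster while active.
; OnActivated hides the mesh and sets player 0's MaxWalkSpeed to 1.5 times the movement component's GetMaxSpeed.
; OnExpired divides GetMaxSpeed by the same factor, writes it back to MaxWalkSpeed, then destroys the actor.
; The boost derives from the current max speed rather than a stored original.
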(event EventOnActivated
  (bind _returnvalue (Game|Player|GetPlayerPawn 0))
  (bind _returnvalue_2 (Actor|GetComponentbyClass _returnvalue "/Script/Engine.CharacterMovementComponent"))
  (Rendering|SetVisibility (Variables|Default|GetStaticMesh) false false)
  (Variables|/Script/Engine.CharacterMovementComponent|SetMaxWalkSpeed _returnvalue_2 (* (Class|MovementComponent|GetMaxSpeed _returnvalue_2) 1.5)))

(event EventOnExpired
  (bind _returnvalue (Game|Player|GetPlayerPawn 0))
  (bind _returnvalue_2 (Actor|GetComponentbyClass _returnvalue "/Script/Engine.CharacterMovementComponent"))
  (Variables|/Script/Engine.CharacterMovementComponent|SetMaxWalkSpeed _returnvalue_2 (/ (Class|MovementComponent|GetMaxSpeed _returnvalue_2) 1.5))
  (Actor|DestroyActor))

(fn ConstructionScript)
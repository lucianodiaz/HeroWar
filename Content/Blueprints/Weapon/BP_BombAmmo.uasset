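; BP_BombAmmo is a timed ammo power-up that temporarily changes the player's current weapon ammo.
; On activation it hides its mesh and passes its Ammo value to ChangeAmmo on the main character's CurrentWeapon.
; On expiry it calls ChangeAmmo with no argument on whatever weapon is current then, and destroys itself.
; Both events find the character by casting player pawn 0 to BP_MainCharacter.
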(event EventOnActivated
  (Rendering|SetVisibility (Variables|Default|GetStaticMesh) false true)
  (bind _asbp_main_character (Utilities|Casting|CastToBP_MainCharacter (Game|Player|GetPlayerPawn 0)))
  (Class|AWeapon|ChangeAmmo (Variables|/Script/HeroWar.MainCharacter|GetCurrentWeapon _asbp_main_character) (Variables|Default|GetAmmo)))

(event EventOnExpired
  (bind _asbp_main_character (Utilities|Casting|CastToBP_MainCharacter (Game|Player|GetPlayerPawn 0)))
  (Class|AWeapon|ChangeAmmo (Variables|/Script/HeroWar.MainCharacter|GetCurrentWeapon _asbp_main_character))
  (Actor|DestroyActor))

(fn ConstructionScript)
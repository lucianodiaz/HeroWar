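; Editor map generator actor that fills a grid with instanced meshes from a selected biome when its build flag is set during construction.
; BuildingWorld matches the biome name, then adds a DimX by DimY grid spaced by Offset from the actor's location, with random height noise.
; A random biome mesh is set on the single instanced component before each instance, so all instances share the last pick.
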(event EventBeginPlay)

(event Collision|EventActorBeginOverlap
  (params (OtherActor :type Actor%20Object%20Reference)))

(event EventTick
  (params (DeltaSeconds :type Float%20%28single-precision%29)))

(fn ConstructionScript
  (if (Variables|Creator|GetStartBulding)
    (CallFunction|BuildingWorld)))

(fn BuildingWorld
  (bind _returnvalue (Transformation|GetActorLocation))
  (for _array_element (Utilities|Struct|BreakBiomes (LocalVariables|GetBiomes))
    (if (Utilities|Enum|Equal(Enum) (.BiomeName (Utilities|Struct|BreakBiome _array_element)) (Variables|Creator|GetSelectBiome))
      (LocalVariables|SetBiome (.MeshBiome (Utilities|Struct|BreakBiome _array_element)))
      (for _index (range 1 (Variables|Creator|GetDimY))
        (LocalVariables|SetYValue _index)
        (for _index_2 (range 1 (Variables|Creator|GetDimX))
          (bind _output_get (LocalVariables|SetXValue _index_2))
          (Components|StaticMesh|SetStaticMesh (Variables|Default|GetInstancedStaticMesh) (Utilities|Array|Get(acopy) (LocalVariables|GetBiome) (Math|Random|RandomIntegerinRange 0 (- (Utilities|Array|Length (LocalVariables|GetBiome)) 1))))
          (Components|InstancedStaticMesh|AddInstance (Variables|Default|GetInstancedStaticMesh) (Math|Transform|MakeTransform (Math|Vector|MakeVector (+ (Math|Conversions|ToFloat(Integer) (* _output_get (LocalVariables|GetOffset))) (.x _returnvalue)) (+ (.y _returnvalue) (Math|Conversions|ToFloat(Integer) (* (LocalVariables|GetYValue) (LocalVariables|GetOffset)))) (+ (.z _returnvalue) (Math|Random|RandomFloatinRange (Variables|Creator|GetNoiseMin) (Variables|Creator|GetNoiseMax)))) "0.000000, 0, 0" "1,1,1")))))))